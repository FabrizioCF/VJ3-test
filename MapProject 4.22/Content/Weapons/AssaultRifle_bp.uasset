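; Automatic assault rifle weapon for the player's ThirdPersonCharacter, with ammo, timed reload and a laser sight.
; Fire starts a looping timer that, while shooting, spends ammo and spawns a Basic_Laser_bp projectile from the muzzle.
; Shots aim at a camera trace impact point with random spread; StopFire clears the timer.
; Tick updates the sight beam, whose target is always the trace end because PickA is false.
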(event Custom|AutomaticFire
  (bind _returnvalue (Game|GetPlayerCharacter 0))
  (bind _ammocount (Variables|Default|GetAmmoCount))
  (bind _returnvalue_2 (> _ammocount 0.0))
  (bind _asthird_person_character (Utilities|Casting|CastToThirdPersonCharacter _returnvalue))
  ;[1 1 1] Fire Method
  (if _returnvalue_2
    (if (and _returnvalue_2 (Variables|/Game/ThirdPersonBP/Blueprints/ThirdPersonCharacter.ThirdPersonCharacter_C|GetIsShooting _asthird_person_character))
      (CallFunction|AmmoCheck)
      (CallFunction|Shoot))
    (else
      (Variables|/Game/ThirdPersonBP/Blueprints/ThirdPersonCharacter.ThirdPersonCharacter_C|SetCanShoot _asthird_person_character false))))

(event EventUnequip
  ;[1 1 1] Unequip Method
  (Variables|/Game/ThirdPersonBP/Blueprints/ThirdPersonCharacter.ThirdPersonCharacter_C|SetActiveWeapon (.AsThird%20Person%20Character (Utilities|Casting|CastToThirdPersonCharacter (Game|GetPlayerCharacter 0))) (Utilities|Struct|MakeGunsData 0 (Variables|Default|GetAmmoCount) (Variables|Default|GetMaxAmmo) (Variables|Default|GetReloadTime) (Variables|Default|GetBulletSpread) (Variables|Default|GetChargeTime))))

(event EventTick
  (params (DeltaSeconds :type Float%20%28single-precision%29))
  (bind _lbs_particle (Variables|Default|GetLBS_particle))
  (bind _laserbeamsight (Variables|Default|GetLaserBeamSight))
  (bind _lbs_particle_2 (Variables|Default|GetLBS_particle))
  (bind _returnvalue (Transformation|GetWorldLocation _laserbeamsight))
  ;[1 1 1] Laser Sight
  (Utilities|IsValid _lbs_particle_2
    (:Is%20Valid
      (Class|ParticleSystemComponent|SetBeamSourcePoint _lbs_particle_2 0 _returnvalue)
      (bind _outhit (Collision|LineTraceByChannel _returnvalue (+ _returnvalue (* (Math|Vector|GetForwardVector (Variables|Default|GetArrow)) 1e+03)) "TraceTypeQuery1" false 0 "None"))
      (Utilities|IsValid _lbs_particle
        (:Is%20Valid
          (Class|ParticleSystemComponent|SetBeamTargetPoint _lbs_particle 0 (Math|Vector|SelectVector (.Location (Collision|BreakHitResult _outhit)) (.TraceEnd (Collision|BreakHitResult _outhit)) false)))))))

(event EventBeginPlay
  ;[1 1 1] Adjunta el componente de LaserSight
  (bind _returnvalue (Effects|SpawnEmitterAttached "/Game/Weapons/LaserSight/LaserBeamSight_PS.LaserBeamSight_PS" (Variables|Default|GetLaserBeamSight) "None"))
  (Variables|Default|SetLBS_particle _returnvalue))

(event EventFire
  (bind _returnvalue (Game|GetPlayerCharacter 0))
  (bind _asthird_person_character (Utilities|Casting|CastToThirdPersonCharacter _returnvalue))
  ;[1 1 1] Fire Method
  (if (> (Variables|Default|GetAmmoCount) 0.0)
    (Variables|/Game/ThirdPersonBP/Blueprints/ThirdPersonCharacter.ThirdPersonCharacter_C|SetCanShoot _asthird_person_character true)
    (CallFunction|AutomaticFire)
    (bind _returnvalue_2 (Utilities|Time|SetTimerbyEvent (delegate Custom|AutomaticFire) (Variables|Default|GetFireRate) true))
    (Variables|Default|SetTimer _returnvalue_2)
    (else
      (Variables|/Game/ThirdPersonBP/Blueprints/ThirdPersonCharacter.ThirdPersonCharacter_C|SetCanShoot _asthird_person_character false))))

(event EventReload
  (bind _returnvalue (Game|GetPlayerCharacter 0))
  (bind _asthird_person_character (Utilities|Casting|CastToThirdPersonCharacter _returnvalue))
  ;[1 1 1] Reload Method
  (if (< (Variables|Default|GetAmmoCount) (Variables|Default|GetMaxAmmo))
    (Utilities|FlowControl|DoOnce false :!label _label
      (:Completed
        (Variables|/Game/ThirdPersonBP/Blueprints/ThirdPersonCharacter.ThirdPersonCharacter_C|SetisReloading _asthird_person_character true)
        (Animation|Montage|MontagePlay (Components|SkeletalMesh|GetAnimInstance (Variables|/Script/Engine.Character|GetMesh _asthird_person_character)) "/Game/FirstPerson/Animations/FirstPersonFire_Montage.FirstPersonFire_Montage" 1.0 "MontageLength" 0.0 true)
        (Components|Animation|PlayAnimation (Variables|Default|Getmesh_sk) "/Game/SciFiWeapDark/Weapons/Anims/Reload_Rifle_Ironsights_w.Reload_Rifle_Ironsights_W" false)
        (Utilities|FlowControl|Delay (Variables|Default|GetReloadTime))
        (Variables|Default|SetAmmoCount (Variables|Default|GetMaxAmmo))
        (Variables|/Game/ThirdPersonBP/Blueprints/ThirdPersonCharacter.ThirdPersonCharacter_C|SetisReloading _asthird_person_character false)
        (goto _label Reset)))))

(event EventStopFire
  ;[1 1 1] Fire Method
  (Utilities|Time|ClearandInvalidateTimerbyHandle (Variables|Default|GetTimer)))

(fn ConstructionScript
  (|CallParentFunction))

(fn AmmoCheck
  (Math|Float|DecrementFloat (Variables|Default|GetAmmoCount)
    (:%20%20
      (Components|Animation|PlayAnimation (Variables|Default|Getmesh_sk) "/Game/SciFiWeapDark/Weapons/Anims/Fire_Rifle_W.Fire_Rifle_W" false)
      (Development|PrintString (Utilities|String|ToString(Float) (Variables|Default|GetAmmoCount))))))

(fn LineTrace
  (bind _returnvalue (Game|GetPlayerCharacter 0))
  (bind _bulletspread (Variables|Default|GetBulletSpread))
  (bind _muzzle (Variables|Default|Getmuzzle))
  (bind _returnvalue_2 (Transformation|GetWorldLocation _muzzle))
  (bind _returnvalue_3 (* _bulletspread -1.0))
  (bind _asthird_person_character (Utilities|Casting|CastToThirdPersonCharacter _returnvalue))
  (bind _returnvalue_4 (Math|Random|RandomFloatinRange _returnvalue_3 _bulletspread))
  (bind _returnvalue_5 (Math|Random|RandomFloatinRange _returnvalue_3 _bulletspread))
  (bind _returnvalue_6 (Math|Random|RandomFloatinRange _returnvalue_3 _bulletspread))
  (bind _followcamera (Variables|/Game/ThirdPersonBP/Blueprints/ThirdPersonCharacter.ThirdPersonCharacter_C|GetFollowCamera _asthird_person_character))
  (bind _returnvalue_7 (Math|Vector|GetForwardVector _followcamera))
  (bind _returnvalue_8 (Transformation|GetWorldLocation _followcamera))
  (bind _returnvalue_9 (* _returnvalue_7 10000))
  (bind _returnvalue_10 (+ _returnvalue_8 _returnvalue_9))
  (bind _returnvalue_11 (+ _returnvalue_10 (Math|Vector|MakeVector _returnvalue_4 _returnvalue_5 _returnvalue_6)))
  (bind _outhit (Collision|LineTraceByChannel _returnvalue_8 _returnvalue_11 "TraceTypeQuery3" false 0 "None" true "(R=0.000000,G=1.000000,B=0.929538,A=1.000000)" "(R=1.000000,G=0.518413,B=0.000000,A=1.000000)" 6.0)) ; GunShot
  (bind _output_get (Variables|Default|SetLaserHitResult _outhit))
  (if true
    (return (Math|Transform|MakeTransform _returnvalue_2 (Math|Rotator|FindLookatRotation _returnvalue_2 (.ImpactPoint (Collision|BreakHitResult _output_get)))))
    (else
      (return (Math|Transform|MakeTransform _returnvalue_2 (Math|Rotator|FindLookatRotation _returnvalue_2 _returnvalue_11))))))

(fn SpawnLaser
  (params (ShootToLocation :type Transform))
  (Game|SpawnActorfromClass "/Game/Weapons/Ammo/Basic_Laser_bp.Basic_Laser_bp_C" ShootToLocation "AlwaysSpawn" 0 0))

(fn Shoot
  (bind _shoottolocation (CallFunction|LineTrace))
  (CallFunction|SpawnLaser _shoottolocation)
  (Components|Animation|PlayAnimation (Variables|Default|Getmesh_sk) "/Game/AnimStarterPack/Fire_Rifle_Hip.Fire_Rifle_Hip" false))