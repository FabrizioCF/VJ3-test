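; Charged laser pistol for the first-person character, with reload and an Unequip that saves its stats to the player's SecondaryWeapon.
; Fire starts a cancellable charge timer, which on completion spends ammo, traces, plays the fire montage, spawns a laser and damages any character hit.
; Aiming uses a spread-randomized camera trace, then a muzzle trace to that impact point, both debug-drawn.
; Reload is DoOnce-guarded and refills ammo after a delay.
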(event Custom|isCharged
  (bind _returnvalue (Game|GetPlayerCharacter 0))
  (bind _asfirst_person_character (Utilities|Casting|CastToFirstPersonCharacter _returnvalue))
  (bind _mesh2p (Variables|/Game/FirstPersonBP/Blueprints/FirstPersonCharacter.FirstPersonCharacter_C|GetMesh2P _asfirst_person_character))
  ;[1 1 1] Fire Method
  (CallFunction|AmmoCheck)
  (bind _outhit (CallFunction|LineTrace))
  (Variables|Default|SetLaserHitResult _outhit)
  (if (Variables|/Game/FirstPersonBP/Blueprints/FirstPersonCharacter.FirstPersonCharacter_C|GetaimDownSight _asfirst_person_character)
    (Animation|Montage|PlayMontage _mesh2p "/Game/FirstPerson/Animations/FirstPersonFire_Montage.FirstPersonFire_Montage"
      (:then
        _))
    (else
      (Animation|Montage|PlayMontage _mesh2p "/Game/FirstPerson/Animations/FirstPersonFire_Montage.FirstPersonFire_Montage" ; Cambiar la animación dependiendo de aimDown
        (:then
          _))))
  (CallFunction|SpawnLaser)
  ;[1 1 1] Daña al jugador
  (bind _asfirst_person_character_2 (Utilities|Casting|CastToFirstPersonCharacter (.hitactor (Variables|Default|GetLaserHitResult))))
  (Default|TakeDamage _asfirst_person_character_2 (Variables|Default|GetDamage)))

(event EventUnequip
  ;[1 1 1] Unequip Method
  (Variables|/Game/FirstPersonBP/Blueprints/FirstPersonCharacter.FirstPersonCharacter_C|SetSecondaryWeapon (.AsFirst%20Person%20Character (Utilities|Casting|CastToFirstPersonCharacter (Game|GetPlayerCharacter 0))) (Utilities|Struct|MakeGunsData "Pistol_bp_C" (Variables|Default|GetAmmoCount) (Variables|Default|GetMaxAmmo) (Variables|Default|GetReloadTime) (Variables|Default|GetBulletSpread) 0.0)))

(event EventClearChargeTimer
  ;[1 1 1] Fire Method
  (Utilities|Time|ClearandInvalidateTimerbyHandle (stale EventFire _returnvalue)))

(event EventReload
  (bind _returnvalue (Game|GetPlayerCharacter 0))
  (bind _asfirst_person_character (Utilities|Casting|CastToFirstPersonCharacter _returnvalue))
  ;[1 1 1] Reload Method
  (if (< (Variables|Default|GetAmmoCount) (Variables|Default|GetMaxAmmo))
    (Utilities|FlowControl|DoOnce false :!label _label
      (:Completed
        (Variables|/Game/FirstPersonBP/Blueprints/FirstPersonCharacter.FirstPersonCharacter_C|SetisReloading _asfirst_person_character true)
        (Animation|Montage|MontagePlay (Components|SkeletalMesh|GetAnimInstance (Variables|/Game/FirstPersonBP/Blueprints/FirstPersonCharacter.FirstPersonCharacter_C|GetMesh2P _asfirst_person_character)) "/Game/FirstPerson/Animations/FirstPersonFire_Montage.FirstPersonFire_Montage" 1.0 "MontageLength" 0.0 true)
        (Components|Animation|PlayAnimation (Variables|Default|Getmesh_sk) "/Game/AnimStarterPack/Reload_Pistol.Reload_Pistol" false)
        (Utilities|FlowControl|Delay (Variables|Default|GetReloadTime))
        (Variables|Default|SetAmmoCount (Variables|Default|GetMaxAmmo))
        (Variables|/Game/FirstPersonBP/Blueprints/FirstPersonCharacter.FirstPersonCharacter_C|SetisReloading _asfirst_person_character false)
        (goto _label Reset)))))

(event EventFire
  ;[1 1 1] Fire Method
  (if (> (Variables|Default|GetAmmoCount) 0.0)
    (bind _returnvalue (Utilities|Time|SetTimerbyEvent (delegate Custom|isCharged) (Variables|Default|GetChargeTime)))
    (Development|PrintString "Estoy cargando")))

(fn ConstructionScript
  (|CallParentFunction))

(fn AmmoCheck
  (Math|Float|DecrementFloat (Variables|Default|GetAmmoCount)
    (:%20%20
      (Components|Animation|PlayAnimation (Variables|Default|Getmesh_sk) "/Game/SciFiWeapDark/Weapons/Anims/Fire_Pistol_W.Fire_Pistol_W" false)
      (Development|PrintString (Utilities|String|ToString(Float) (Variables|Default|GetAmmoCount))))))

(fn LineTrace
  (bind _returnvalue (Game|GetPlayerCharacter 0))
  (bind _bulletspread (Variables|Default|GetBulletSpread))
  (bind _returnvalue_2 (* _bulletspread -1.0))
  (bind _asfirst_person_character (Utilities|Casting|CastToFirstPersonCharacter _returnvalue))
  (bind _firstpersoncamera (Variables|/Game/FirstPersonBP/Blueprints/FirstPersonCharacter.FirstPersonCharacter_C|GetFirstPersonCamera _asfirst_person_character))
  (bind _returnvalue_3 (Transformation|GetWorldLocation _firstpersoncamera))
  (bind _outhit (Collision|LineTraceByChannel _returnvalue_3 (+ (+ _returnvalue_3 (* (Math|Vector|GetForwardVector _firstpersoncamera) 10000)) (Math|Vector|MakeVector (Math|Random|RandomFloatinRange _returnvalue_2 _bulletspread) (Math|Random|RandomFloatinRange _returnvalue_2 _bulletspread) (Math|Random|RandomFloatinRange _returnvalue_2 _bulletspread))) "TraceTypeQuery2" false 0 "ForDuration" true "(R=1.000000,G=0.000000,B=0.000000,A=1.000000)" "(R=0.000000,G=1.000000,B=0.000000,A=1.000000)" 6.0)) ; CameraShot
  (bind _outhit_2 (Collision|LineTraceByChannel (Transformation|GetWorldLocation (Variables|Default|Getmuzzle)) (.ImpactPoint (Collision|BreakHitResult _outhit)) "TraceTypeQuery1" false 0 "ForDuration" true "(R=0.000000,G=1.000000,B=0.929538,A=1.000000)" "(R=0.000000,G=1.000000,B=0.000000,A=1.000000)" 6.0)) ; GunShot
  (return _outhit_2))

(fn SpawnLaser
  (Game|SpawnActorfromClass "/Game/Weapons/Ammo/Basic_Laser_bp.Basic_Laser_bp_C" (Math|Transform|MakeTransform (Transformation|GetWorldLocation (Variables|Default|Getmuzzle)) (Camera|GetCameraRotation (Variables|/Script/Engine.PlayerController|GetPlayerCameraManager (Game|GetPlayerController 0)))) "AlwaysSpawn" 0 0))