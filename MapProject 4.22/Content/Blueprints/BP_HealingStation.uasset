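; Healing station that heals the player character while it stands inside the capsule trigger, drawing on a limited healing capacity.
; Capsule overlaps track affected players and toggle the particle effect.
; Tick applies a fixed per-frame heal, and once capacity empties it locks into recharging at a tenth of that rate until full.
; A dynamic emissive material shows idle, healing and recharging states through color, intensity and frequency.
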(event OnComponentBeginOverlap(Capsule)
  (params (OverlappedComponent :type Primitive%20Component%20Object%20Reference) (OtherActor :type Actor%20Object%20Reference) (OtherComp :type Primitive%20Component%20Object%20Reference) (OtherBodyIndex :type Integer) (bFromSweep :type Boolean) (SweepResult :type Hit%20Result%20Structure%20%28by%20ref%29))
  (if (== OtherActor (Game|GetPlayerCharacter 0))
    (bind _asthird_person_character (Utilities|Casting|CastToThirdPersonCharacter OtherActor))
    (Utilities|Array|Add (Variables|Default|GetPlayersAffected) _asthird_person_character)
    (Variables|Default|SetIsServicing? true)
    (CallFunction|CustomEvent)))

(event OnComponentEndOverlap(Capsule)
  (params (OverlappedComponent :type Primitive%20Component%20Object%20Reference) (OtherActor :type Actor%20Object%20Reference) (OtherComp :type Primitive%20Component%20Object%20Reference) (OtherBodyIndex :type Integer))
  (bind _playersaffected (Variables|Default|GetPlayersAffected))
  (if (== OtherActor (Game|GetPlayerCharacter 0))
    (bind _asthird_person_character (Utilities|Casting|CastToThirdPersonCharacter OtherActor))
    (Utilities|Array|RemoveItem _playersaffected _asthird_person_character)
    (if (== (Utilities|Array|Length _playersaffected) 0)
      (Variables|Default|SetIsServicing? false)
      (CallFunction|CustomEvent0))))

(event Custom|CustomEvent
  (Components|Activation|SetActive (Variables|Default|GetParticleSystem) true false))

(event Custom|CustomEvent_0
  (Components|Activation|SetActive (Variables|Default|GetParticleSystem) false true))

(event Collision|EventActorBeginOverlap
  (params (OtherActor :type Actor%20Object%20Reference)))

(event EventTick
  (params (DeltaSeconds :type Float%20%28single-precision%29))
  (bind _emissive_material (Variables|Default|GetEmissive%20Material))
  (bind _emissive_material_2 (Variables|Default|GetEmissive%20Material))
  (if (and (not (Variables|Default|GetIsRecharging?)) (> (Variables|Default|GetHealingCapacity) 0.0))
    (if (and (Variables|Default|GetIsServicing?) (Variables|Default|GetIsOn?))
      (for _array_element (Variables|Default|GetPlayersAffected)
        (Default|Heal _array_element (Variables|Default|GetHealingAmount))
        (Variables|Default|SetHealingCapacity (Math|Float|Clamp(Float) (- (Variables|Default|GetHealingCapacity) (Variables|Default|GetHealingAmount)) 0.0 (Variables|Default|GetHealingCapacity)))
        (Rendering|Material|SetScalarParameterValue _emissive_material_2 "Frequency" 2.0 :!class /Script/Engine.MaterialInstanceDynamic)
        (Rendering|Material|SetScalarParameterValue _emissive_material_2 "Intensity" 0.5 :!class /Script/Engine.MaterialInstanceDynamic)
        (Rendering|Material|SetVectorParameterValue _emissive_material_2 "LightColor" "(R=0.000000,G=255.000000,B=21.957472,A=1.000000)" :!class /Script/Engine.MaterialInstanceDynamic))
      (else
        (Rendering|Material|SetScalarParameterValue _emissive_material "Frequency" 0.5 :!class /Script/Engine.MaterialInstanceDynamic)
        (Rendering|Material|SetScalarParameterValue _emissive_material "Intensity" 0.1 :!class /Script/Engine.MaterialInstanceDynamic)
        (Rendering|Material|SetVectorParameterValue _emissive_material "LightColor" "(R=0.000000,G=255.000000,B=253.426453,A=1.000000)" :!class /Script/Engine.MaterialInstanceDynamic)))
    (else
      (Variables|Default|SetIsRecharging? true)
      (Rendering|Material|SetScalarParameterValue (Variables|Default|GetEmissive%20Material) "Intensity" 0.0 :!class /Script/Engine.MaterialInstanceDynamic)
      (Variables|Default|SetHealingCapacity (Math|Float|Clamp(Float) (+ (Variables|Default|GetHealingCapacity) (/ (Variables|Default|GetHealingAmount) 1e+01)) 0.0 (Variables|Default|GetMaxHealingCapacity)))
      (if (== (Variables|Default|GetHealingCapacity) (Variables|Default|GetMaxHealingCapacity))
        (Variables|Default|SetIsOn? true)
        (Variables|Default|SetIsRecharging? false)))))

(fn ConstructionScript
  (Variables|Default|SetHealingCapacity (Variables|Default|GetMaxHealingCapacity))
  (bind _returnvalue (Rendering|Material|CreateDynamicMaterialInstance (Variables|Default|GetHealingStation) 4 "/Game/Exported/HealingPlatform/M_HealingStationEmission.M_HealingStationEmission" "EmissiveMaterial" :!class /Script/Engine.PrimitiveComponent))
  (bind _output_get (Variables|Default|SetEmissive%20Material _returnvalue))
  (Rendering|Material|SetVectorParameterValue _output_get "LightColor" "(R=0.000000,G=255.000000,B=253.426453,A=1.000000)" :!class /Script/Engine.MaterialInstanceDynamic)
  (Rendering|Material|SetScalarParameterValue _output_get "Intensity" 0.1 :!class /Script/Engine.MaterialInstanceDynamic))