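; World-space health bar actor with a text label and a holographic bar, turned each tick to oppose the first player's yaw.
; SetValues writes replicated Text, Value and MaxValue, whose OnRep functions update the label and scale the bar by health ratio.
; A dynamic hologram material tints from red to green through HSV interpolation.
; OnRep_Color applies named color presets, and healing state switches Color between green and cyan.
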(event Custom|SetValues
  (params (Text :type Text) (Value :type Float%20%28single-precision%29) (MaxValue :type Float%20%28single-precision%29))
  (Variables|Default|SetText Text)
  (Variables|Default|SetMaxValue MaxValue)
  (Variables|Default|SetValue Value))

(event EventTick
  (params (DeltaSeconds :type Float%20%28single-precision%29))
  (bind _returnvalue (Game|GetPlayerController 0))
  (Utilities|IsValid _returnvalue
    (:Is%20Valid
      (Transformation|SetWorldRotation (Variables|Default|GetDefaultSceneRoot) (Math|Rotator|MakeRotator 0.0 0.0 (+ (.Yaw (Math|Rotator|BreakRotator (.rotation (Transformation|GetActorTransform _returnvalue)))) -1.8e+02)) false false))))

(fn ConstructionScript
  (bind _returnvalue (Rendering|Material|CreateDynamicMaterialInstance (Variables|Default|GetBarCube) 0 "/Game/M_Hologram.M_Hologram" "HolographicMaterial" :!class /Script/Engine.PrimitiveComponent))
  (bind _output_get (Variables|Default|SetHolographicMaterial _returnvalue))
  (Rendering|Material|SetVectorParameterValue _output_get "Color" "(R=0.000000,G=3.193452,B=5.000000,A=1.000000)" :!class /Script/Engine.MaterialInstanceDynamic))

(fn CalculateValue
  (params (CurrentValue :type Float%20%28single-precision%29) (MaxValue :type Float%20%28single-precision%29))
  (bind _returnvalue (/ CurrentValue MaxValue))
  (bind _barscene (Variables|Default|GetBarScene))
  (bind _returnvalue_2 (Transformation|GetWorldScale _barscene))
  (Transformation|SetWorldScale3D _barscene (Math|Vector|MakeVector (.x _returnvalue_2) (/ _returnvalue 2.0) (.z _returnvalue_2)))
  (CallFunction|ChangeColor (Class|KismetMathLibrary|LinearColorLerpUsingHSV (LocalVariables|GetRed) (LocalVariables|GetGreen) _returnvalue)))

(fn ChangeColor
  (params (Color :type Linear%20Color%20Structure))
  (Rendering|Material|SetVectorParameterValue (Variables|Default|GetHolographicMaterial) "Color" Color :!class /Script/Engine.MaterialInstanceDynamic))

(fn OnRepValue
  (CallFunction|CalculateValue (Variables|Default|GetValue) (Variables|Default|GetMaxValue)))

(fn OnRepText
  (Rendering|Components|TextRender|SetText (Variables|Default|GetTextRender) (Variables|Default|GetText)))

(fn OnRepColor
  (switch name (Variables|Default|GetColor)
    (:Default
      _)
    (:Green
      (Class|KismetMathLibrary|LinearColorSetfromHSV (LocalVariables|GetColorHex) 112.0 1.0 2e+01 1.0))
    (:Blue
      (Class|KismetMathLibrary|LinearColorSetfromHSV (LocalVariables|GetColorHex) 2.3e+02 1.0 2e+01 1.0))
    (:Cyan
      (Class|KismetMathLibrary|LinearColorSetfromHSV (LocalVariables|GetColorHex) 1.9e+02 1.0 2e+01 1.0))
    (:Yellow
      (Class|KismetMathLibrary|LinearColorSetfromHSV (LocalVariables|GetColorHex) 58.0 1.0 2e+01 1.0))
    (:Red
      (Class|KismetMathLibrary|LinearColorSetfromHSV (LocalVariables|GetColorHex) 359.0 1.0 2e+01 1.0)))
  (CallFunction|ChangeColor (LocalVariables|GetColorHex)))

(fn OnRepIsHealing
  (if (Variables|Default|GetIsHealing)
    (Variables|Default|SetColor "Green")
    (else
      (Variables|Default|SetColor "Cyan"))))

(fn OnRepIsDamaged)