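; Energy cell pickup that raises one of the player's gun attribute multipliers (damage, cooldown or fire rate) when touched, then destroys itself.
; The construction script derives the bonus value and mesh scale from the big-cell flag and picks the emissive material by type.
; Entering the Range trigger plays a timeline that magnetically pulls the cell toward the player, interpolating location plus a track offset and updating rotation via look-at.
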(event OnComponentBeginOverlap(Range)
  (params (OverlappedComponent :type Primitive%20Component%20Object%20Reference) (OtherActor :type Actor%20Object%20Reference) (OtherComp :type Primitive%20Component%20Object%20Reference) (OtherBodyIndex :type Integer) (bFromSweep :type Boolean) (SweepResult :type Hit%20Result%20Structure%20%28by%20ref%29))
  ;[1 1 1] If a Player Character is Touching...
  (if (== OtherActor (Game|GetPlayerCharacter 0))
    (bind _msgnetictrack (Timeline|Magnetic%20Timeline PlayFromStart)
      (:Update
        (CallFunction|FlyTowardsPicker _msgnetictrack)))))

(event OnComponentBeginOverlap(EnergyCell)
  (params (OverlappedComponent :type Primitive%20Component%20Object%20Reference) (OtherActor :type Actor%20Object%20Reference) (OtherComp :type Primitive%20Component%20Object%20Reference) (OtherBodyIndex :type Integer) (bFromSweep :type Boolean) (SweepResult :type Hit%20Result%20Structure%20%28by%20ref%29))
  (if (== OtherActor (Game|GetPlayerCharacter 0))
    (bind _asthird_person_character (Utilities|Casting|CastToThirdPersonCharacter (Game|GetPlayerCharacter 0)))
    (Default|AddtoGunAttributeMultiplier _asthird_person_character (Variables|Default|GetType) (Variables|Default|GetValue))
    (Actor|DestroyActor)))

(event EventBeginPlay)

(event Collision|EventActorBeginOverlap
  (params (OtherActor :type Actor%20Object%20Reference)))

(event EventTick
  (params (DeltaSeconds :type Float%20%28single-precision%29)))

(fn ConstructionScript
  (bind _energycell (Variables|Default|GetEnergyCell))
  (if (Variables|Default|GetIsBig?)
    (Variables|Default|SetValue (+ (Variables|Default|GetDefaultValue) (* (Variables|Default|GetDefaultValue) (Variables|Default|GetBigValueBonus))))
    (Transformation|SetRelativeScale3D _energycell (* (Variables|/Script/Engine.SceneComponent|GetRelativeScale3D _energycell) (+ (/ (Variables|Default|GetBigValueBonus) 2.0) (Variables|Default|GetDefaultValue))))
    (else
      (Variables|Default|SetValue (Variables|Default|GetDefaultValue))))
  (switch name (Variables|Default|GetType)
    (:Default
      (Variables|Default|SetType "FireRate"))
    (:Damage
      (Variables|Default|SetEmissiveMaterial "/Game/Exported/EnergyCell/M_EnergyCell_Red.M_EnergyCell_Red"))
    (:Cooldown
      (Variables|Default|SetEmissiveMaterial "/Game/Exported/EnergyCell/M_EnergyCell.M_EnergyCell"))
    (:FireRate
      (Variables|Default|SetEmissiveMaterial "/Game/Exported/EnergyCell/M_EnergyCell_Yellow.M_EnergyCell_Yellow")))
  (Rendering|Material|SetMaterial (Variables|Default|GetEnergyCell) 0 (Variables|Default|GetEmissiveMaterial)))

(fn FlyTowardsPicker
  (params (TrackUpdate :type Vector))
  ;[1 1 1] Calculation of flight.
  (LocalVariables|SetActorInitialLocation (Transformation|GetActorLocation (Game|GetPlayerCharacter 0)))
  ;[1 1 1] Generate translation numbers.
  (LocalVariables|SetNewLocation (+ TrackUpdate (Math|Interpolation|VInterpTo (.Location (Math|Transform|BreakTransform (Transformation|GetActorTransform))) (LocalVariables|GetActorInitialLocation) (Utilities|Time|GetWorldDeltaSeconds) (Variables|Default|GetPickupSpeed))))
  ;[1 1 1] Generate rotation numbers.
  (LocalVariables|SetNewRotation (Math|Rotator|FindLookatRotation (LocalVariables|GetActorInitialLocation) (Math|Vector|MakeVector (.X (Math|Vector|BreakVector (LocalVariables|GetNewLocation))) (.Y (Math|Vector|BreakVector (LocalVariables|GetNewLocation))) (+ (.Z (Math|Vector|BreakVector (LocalVariables|GetNewLocation))) (.SphereRadius (Collision|GetComponentBounds (Variables|/Script/Engine.Character|GetMesh (Game|GetPlayerCharacter 0))))))))
  ;[1 1 1] Set location.
  (Transformation|SetActorLocation (LocalVariables|GetNewLocation) false false)
  ;[1 1 1] Set Rotation.
  (Transformation|SetActorRotation (LocalVariables|GetNewRotation)))