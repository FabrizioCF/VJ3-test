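; BP_ItemSpawner is a spawner actor that places a BP_EnergyCell in the level when play begins.
; SpawnEnergyCell casts Item to the energy cell class, stopping if that fails, and spawns it at the Sphere component's transform with the spawner's Type and IsBig values.
; It then raises the cell's root along local Z by a multiple of the EnergyCell component's bounds radius, so the offset scales with cell size.
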(event EventBeginPlay
  (CallFunction|SpawnEnergyCell))

(event Collision|EventActorBeginOverlap
  (params (OtherActor :type Actor%20Object%20Reference)))

(event EventTick
  (params (DeltaSeconds :type Float%20%28single-precision%29)))

(fn ConstructionScript)

(fn SpawnEnergyCell
  (bind _asbp_energy_cell (Utilities|Casting|CastToBP_EnergyCellClass (Variables|Default|GetItem)))
  (bind _returnvalue (Game|SpawnActorfromClass _asbp_energy_cell (Transformation|GetWorldTransform (Variables|Default|GetSphere)) "Undefined" 0 (Variables|Default|GetType) (Variables|Default|GetIsBig?) 0))
  (Class|SceneComponent|AddLocalTransform (Variables|/Game/Blueprints/BP_EnergyCell.BP_EnergyCell_C|GetDefaultSceneRoot _returnvalue) (Math|Transform|MakeTransform (Math|Vector|MakeVector 0.0 0.0 (* (.SphereRadius (Collision|GetComponentBounds (Variables|/Game/Blueprints/BP_EnergyCell.BP_EnergyCell_C|GetEnergyCell _returnvalue))) 1.25)) "0, 0, 0" "1,1,1") false true))