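; BP_Spawner is a spawn point that spawns a randomly raffled object class at its own transform.
; SpawnerRaffle filters the weighted class map by approval flags and player-start eligibility, then picks a forced class or draws by ticket weight.
; SpawnObject creates the drawn class, tagging any PlayerStart with its player index.
; UnoverlapTranslate can lift the spawned actor by its bounds height, with special handling for energy cells.
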(event Custom|Event%20SpawnerRaffle
  (params (CanProducePlayers? :type Boolean) (ForceDraw :type Actor%20Class%20Reference))
  (bind _index (CallFunction|SpawnerTypeRaffle CanProducePlayers? ForceDraw))
  (bind _output_get (Variables|Default|SetObjectIndex _index))
  (bind _keys (Utilities|Map|Keys (Variables|Default|GetObjectBuffer)))
  (Variables|Default|SetSpawnerType (Utilities|String|StringToName (Utilities|GetClassDisplayName (Utilities|Array|Get(acopy) _keys _output_get)))))

(event Custom|Event%20SpawnObject
  (params (PlayerIndex :type Integer) (MaxPlayerCount :type Integer))
  (CallFunction|SpawnObject (Variables|Default|GetObjectIndex) PlayerIndex))

(event Collision|EventActorBeginOverlap
  (params (OtherActor :type Actor%20Object%20Reference)))

(event EventTick
  (params (DeltaSeconds :type Float%20%28single-precision%29)))

(fn ConstructionScript)

(fn UnoverlapTranslate
  (bind _spawnedactor (Variables|Default|GetSpawnedActor))
  (bind _returnvalue (Transformation|GetActorLocation _spawnedactor))
  (bind (_x _y _z) (Math|Vector|BreakVector _returnvalue))
  (if (Math|Vector|Equal(Vector) (.Origin (Collision|GetActorBounds (Variables|Default|GetSpawnedActor) false)) (Transformation|GetActorLocation) 0.01)
    (if (== (Utilities|GetClass _spawnedactor) "/Game/Blueprints/BP_EnergyCell.BP_EnergyCell_C")
      (bind _asbp_energy_cell (Utilities|Casting|CastToBP_EnergyCell _spawnedactor))
      (LocalVariables|SetDestinedLocation (Math|Vector|MakeVector _x _y (+ (.Z (Math|Vector|BreakVector (.BoxExtent (Collision|GetComponentBounds (Variables|/Game/Blueprints/BP_EnergyCell.BP_EnergyCell_C|GetEnergyCell _asbp_energy_cell))))) _z)))
      (else
        (LocalVariables|SetDestinedLocation (Math|Vector|MakeVector _x _y (+ (.Z (Math|Vector|BreakVector (.BoxExtent (Collision|GetActorBounds _spawnedactor true)))) _z)))))
    (Transformation|Teleport _spawnedactor (LocalVariables|GetDestinedLocation) "0, 0, 0")))

(fn SpawnerTypeRaffle
  (params (CanProducePlayer? :type Boolean) (ForceDraw :type Actor%20Class%20Reference))
  (bind _isapprovedspawn_ (Variables|Default|GetIsApprovedSpawn?))
  (Variables|Default|SetObjectBuffer (Variables|Default|GetObjectProbability))
  (bind _values (Utilities|Map|Values _isapprovedspawn_))
  (for (_array_element _array_index) _values
    (if _array_element
      (if (not CanProducePlayer?)
        (Utilities|Map|Remove (Variables|Default|GetObjectBuffer) "/Script/Engine.PlayerStart"))
      (else
        (bind _keys (Utilities|Map|Keys _isapprovedspawn_))
        (Utilities|Map|Remove (Variables|Default|GetObjectBuffer) (Utilities|Array|Get(acopy) _keys _array_index)))))
  (bind _keys_2 (Utilities|Map|Keys (Variables|Default|GetObjectBuffer)))
  (if (Utilities|Array|IsValidIndex _keys_2)
    (if (Utilities|IsValidClass ForceDraw)
      (bind _keys_3 (Utilities|Map|Keys (Variables|Default|GetObjectBuffer)))
      (return (Utilities|Array|FindItem _keys_3 ForceDraw))
      (else
        (bind _values_2 (Utilities|Map|Values (Variables|Default|GetObjectBuffer)))
        (for _array_element_2 _values_2
          (LocalVariables|SetSpawnerTypeTickets (+ _array_element_2 (LocalVariables|GetSpawnerTypeTickets))))
        (LocalVariables|SetDrawedNumber (Math|Random|RandomIntegerinRange 0 (- (LocalVariables|GetSpawnerTypeTickets) 1)))
        (bind _values_3 (Utilities|Map|Values (Variables|Default|GetObjectBuffer)))
        (bind (_array_element_3 _array_index_2) (Utilities|Array|ForEachLoopwithBreak _values_3 :!label _label)
          (:LoopBody
            (LocalVariables|SetIsInRange? (Math|Integer|InRange(Integer) (LocalVariables|GetDrawedNumber) (LocalVariables|GetSnowballNumber) (+ (LocalVariables|GetSnowballNumber) _array_element_3) true false))
            (LocalVariables|SetSnowballNumber (+ _array_element_3 (LocalVariables|GetSnowballNumber)))
            (if (LocalVariables|GetIsInRange?)
              (LocalVariables|SetSelectedIndex _array_index_2)
              (goto _label Break)))
          (:Completed
            (return (LocalVariables|GetSelectedIndex))))))
    (else
      (bind _output_get (Variables|Default|SetObjectIndex -1))
      (return _output_get))))

(fn SpawnObject
  (params (ObjectIndex :type Integer) (PlayerIndex :type Integer))
  ;[1 1 1] From the raffled index, create get the specified object class.
  (bind _keys (Utilities|Map|Keys (Variables|Default|GetObjectBuffer)))
  ;[1 1 1] Create the actor and give the spawner's position to it.
  (bind _returnvalue (Game|SpawnActorfromClass (Utilities|Array|Get(acopy) _keys ObjectIndex) (Transformation|GetActorTransform) "Undefined" 0 0))
  (bind _output_get (Variables|Default|SetSpawnedActor _returnvalue))
  (if (== (Utilities|GetClass _output_get) "/Script/Engine.PlayerStart")
    (bind _asplayer_start (Utilities|Casting|CastToPlayerStart (Variables|Default|GetSpawnedActor)))
    (Variables|/Script/Engine.PlayerStart|SetPlayerStartTag _asplayer_start (Utilities|String|StringToName (Utilities|String|ToString(Integer) PlayerIndex)))))