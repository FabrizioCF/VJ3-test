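; BP_Counter is a world-space counter actor that displays a label and a value with an "x" suffix.
; Construction sets both texts and picks a red, yellow or blue Poppins material from Color, defaulting to blue.
; Tick yaws the root opposite the first player controller's rotation so the text faces that player.
; SetValues stores new data, ChangeValue updates value text, and RepNotifies refresh text, though OnRep_Value omits the suffix; ChangeColor is empty.
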(event Custom|SetValues
  (params (Label :type Text) (Value :type Text))
  (Variables|Default|SetLabel Label)
  (Variables|Default|SetValue Value))

(event EventTick
  (params (DeltaSeconds :type Float%20%28single-precision%29))
  (bind _returnvalue (Game|GetPlayerController 0))
  (Utilities|IsValid _returnvalue
    (:Is%20Valid
      (Transformation|SetWorldRotation (Variables|Default|GetDefaultSceneRoot) (Math|Rotator|MakeRotator 0.0 0.0 (+ (.Yaw (Math|Rotator|BreakRotator (.rotation (Transformation|GetActorTransform _returnvalue)))) -1.8e+02)) false false))))

(fn ConstructionScript
  (Rendering|Components|TextRender|SetText (Variables|Default|GetLabelText) (Variables|Default|GetLabel))
  (Rendering|Components|TextRender|SetText (Variables|Default|GetValueText) (Utilities|Text|ToText(String) (Utilities|String|Append (Utilities|String|ToString(Text) (Variables|Default|GetValue)) "x")))
  (switch name (Variables|Default|GetColor)
    (:Default
      (Class|TextRenderComponent|SetTextMaterial (Variables|Default|GetLabelText) "/Game/EngineMaterials/M_PoppinsBlue.M_PoppinsBlue" :!label _label))
    (:Red
      (Class|TextRenderComponent|SetTextMaterial (Variables|Default|GetLabelText) "/Game/EngineMaterials/M_PoppinsRed.M_PoppinsRed"))
    (:Yellow
      (Class|TextRenderComponent|SetTextMaterial (Variables|Default|GetLabelText) "/Game/EngineMaterials/M_PoppinsYellow.M_PoppinsYellow"))
    (:Blue
      (goto _label))))

(fn ChangeValue
  (params (Value :type Text))
  (bind _output_get (Variables|Default|SetValue Value))
  (Rendering|Components|TextRender|SetText (Variables|Default|GetValueText) (Utilities|Text|ToText(String) (Utilities|String|Append (Utilities|String|ToString(Text) _output_get) "x"))))

(fn ChangeColor)

(fn OnRepLabel
  (Rendering|Components|TextRender|SetText (Variables|Default|GetLabelText) (Variables|Default|GetLabel)))

(fn OnRepValue
  (Rendering|Components|TextRender|SetText (Variables|Default|GetValueText) (Variables|Default|GetValue)))